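; Player character Blueprint with axis-driven movement and look, plus picking up and dropping physics objects.
; The Coger input toggles between grabbing and releasing, tracked by Estacogiendoobjeto.
; Grabbing line-traces a short distance from the camera and attaches a physics-simulating hit component to the PhysicsHandle.
; Tick keeps the handle's target at the Loc.objeto component, so the held object follows that point.
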(event Custom|Coger%20objeto
  (bind _returnvalue (Game|GetPlayerCameraManager 0))
  (bind _returnvalue_2 (Transformation|GetActorLocation _returnvalue))
  ;[1 1 1] Coger y soltar objetos
  (bind _outhit (Collision|LineTraceByChannel _returnvalue_2 (+ (* (Transformation|GetActorForwardVector _returnvalue) 300) _returnvalue_2) "TraceTypeQuery1" false 0 "None"))
  (if true
    (if (Physics|IsSimulatingPhysics (.HitComponent (Collision|BreakHitResult _outhit)) "None")
      (Class|PhysicsHandleComponent|GrabComponentatLocation (Variables|Default|GetPhysicsHandle) (.HitComponent (Collision|BreakHitResult _outhit)) "None" (Transformation|GetWorldLocation (.HitComponent (Collision|BreakHitResult _outhit))))
      (Variables|Default|Setestacogiendoobjeto true))))

(event Custom|soltar%20objeto
  ;[1 1 1] Coger y soltar objetos
  (Physics|Components|PhysicsHandle|ReleaseComponent (Variables|Default|GetPhysicsHandle))
  (Variables|Default|Setestacogiendoobjeto false))

(event EventTick
  (params (DeltaSeconds :type Float%20%28single-precision%29))
  ;[1 1 1] Coger y soltar objetos
  (Physics|Components|PhysicsHandle|SetTargetLocation (Variables|Default|GetPhysicsHandle) (Transformation|GetWorldLocation (Variables|Default|Getloc.objeto))))

(event Input|ActionEvents|InputActionCoger
  (params (Key :type Key%20Structure :default "None"))
  ;[1 1 1] Coger y soltar objetos
  (:Pressed
    (if (Variables|Default|Getestacogiendoobjeto)
      (CallFunction|SoltarObjeto)
      (else
        (CallFunction|CogerObjeto)))))

(event Input|AxisEvents|InputAxisMoveForward
  (params (AxisValue :type Float%20%28single-precision%29))
  ;[1 1 1] Movimiento
  (Pawn|Input|AddMovementInput (Math|Vector|GetForwardVector (Pawn|GetControlRotation :!class /Script/Engine.Pawn)) AxisValue false))

(event Input|AxisEvents|InputAxisMove_Right
  (params (AxisValue :type Float%20%28single-precision%29))
  ;[1 1 1] Movimiento
  (Pawn|Input|AddMovementInput (Math|Vector|GetRightVector (Pawn|GetControlRotation :!class /Script/Engine.Pawn)) AxisValue false))

(event Input|AxisEvents|InputAxisTurn
  (params (AxisValue :type Float%20%28single-precision%29))
  ;[1 1 1] Movimiento
  (Pawn|Input|AddControllerYawInput AxisValue))

(event Input|AxisEvents|InputAxisLook_Up
  (params (AxisValue :type Float%20%28single-precision%29))
  ;[1 1 1] Movimiento
  (Pawn|Input|AddControllerPitchInput AxisValue))

(fn ConstructionScript)